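; Microwave Blueprint with an Open/Close event that swings a part, presumably the door, for the first-person player.
; The event gets the target from the player character's ObjectMessage and tests its attach parent's truncated world yaw to pick a direction.
; At the -90 position it plays a bell sound and runs a timeline driving the parent's relative yaw, otherwise it reverses that timeline.
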(event Collision|EventActorBeginOverlap
  (params (OtherActor :type Actor%20Object%20Reference)))

(event EventTick
  (params (DeltaSeconds :type Float%20%28single-precision%29)))

(event EventOpen/Close
  (Utilities|FlowControl|Sequence
    (:then_0
      (bind _asfirst_person_character (Utilities|Casting|CastToFirstPersonCharacter (Game|GetPlayerCharacter 0)))
      (bind _door (Class|Variable|Object(Message) _asfirst_person_character))
      (Variables|Default|SetTarget _door))
    (:then_1
      (if (== (Math|Float|Truncate (.yaw (Transformation|GetWorldRotation (Transformation|GetAttachParent (Variables|Default|GetTarget))))) -90)
        (Audio|PlaySoundatLocation "/Game/ToJamAudio/soundEffect/microwave_bell_Sound_Cue.microwave_bell_Sound_Cue" (Transformation|GetWorldLocation (Variables|Default|GetMicrowave)) "0, 0, 0" 1.0 1.0 0.0 0 0 0)
        (bind _newtrack_0 (Timeline|Timeline_0 PlayFromStart)
          (:Update
            (Transformation|SetRelativeRotation (Transformation|GetAttachParent (Variables|Default|GetTarget)) (Math|Rotator|MakeRotator 0.0 0.0 _newtrack_0) false false)))
        (else
          (Timeline|Timeline_0 ReverseFromEnd))))))

(fn ConstructionScript)

(fn Object
  (return 0))