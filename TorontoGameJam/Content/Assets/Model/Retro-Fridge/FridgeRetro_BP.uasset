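; Retro fridge Blueprint whose Open/Close event swings a part open or closed, likely the door the player targets.
; The event asks the first-person character for its targeted object through ObjectMessage and acts on that object's attach parent.
; A timeline drives the parent's relative yaw, playing forward when its world yaw truncates to 90 and reversing from the end otherwise.
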(event EventBeginPlay)

(event EventOpen/Close
  (Utilities|FlowControl|Sequence
    (:then_0
      (bind _asfirst_person_character (Utilities|Casting|CastToFirstPersonCharacter (Game|GetPlayerCharacter 0)))
      (bind _door (Class|Variable|Object(Message) _asfirst_person_character))
      (Variables|Default|SetTarget _door))
    (:then_1
      (if (== 90 (Math|Float|Truncate (.yaw (Transformation|GetWorldRotation (Transformation|GetAttachParent (Variables|Default|GetTarget))))))
        (bind _newtrack_0 (Timeline|Open/close%20timeline PlayFromStart)
          (:Update
            (Transformation|SetRelativeRotation (Transformation|GetAttachParent (Variables|Default|GetTarget)) (Math|Rotator|MakeRotator 0.0 0.0 _newtrack_0) false false)))
        (else
          (Timeline|Open/close%20timeline ReverseFromEnd))))))

(event EventTick
  (params (DeltaSeconds :type Float%20%28single-precision%29)))

(fn ConstructionScript)

(fn Object
  (return 0))