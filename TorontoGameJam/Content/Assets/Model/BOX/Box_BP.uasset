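; Box Blueprint that collects overlapping pick-up actors and keeps a count of them.
; On begin overlap, it checks the other actor's root component for the "Pick Up" tag.
; A match plays the collect sound at the FirstPersonCharacter's location, destroys the overlapping actor and increments the Item counter.
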(event EventBeginPlay)

(event EventTick
  (params (DeltaSeconds :type Float%20%28single-precision%29)))

(event Collision|EventActorBeginOverlap
  (params (OtherActor :type Actor%20Object%20Reference))
  (bind _returnvalue (Actor|GetActorOfClass "/Game/FirstPersonBP/Blueprints/FirstPersonCharacter.FirstPersonCharacter_C"))
  (if (Components|ComponentHasTag (Variables|/Script/Engine.Actor|GetRootComponent OtherActor) "Pick Up")
    (Audio|PlaySoundatLocation "/Game/ToJamAudio/soundEffect/collect_Cue.collect_Cue" (Transformation|GetWorldLocation (Variables|/Script/Engine.Actor|GetRootComponent _returnvalue)) "0, 0, 0" 1.0 1.0 0.0 0 0 0)
    (Actor|DestroyActor OtherActor)
    (Variables|Default|SetItem (+ (Variables|Default|GetItem) 1))))

(fn ConstructionScript)